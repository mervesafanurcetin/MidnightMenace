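; BP_Drawer is an interactable drawer with a door that moves the player in and out of it.
; Each Interact toggles the Inside flag and teleports player character 0 to the REFInside or REFOutside transform, matching location and rotation.
; The Door snaps to a narrower angle when the player enters and a wider one on exit, with no animation.
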(event `/Game/Blueprints/BPI_Interaction.Interact`
  (bind (_returnvalue_location _returnvalue_rotation) (`KismetMathLibrary.BreakTransform` (`SceneComponent.K2_GetComponentToWorld` (`self.REF Inside`))))
  (bind (_returnvalue_location_2 _returnvalue_rotation_2) (`KismetMathLibrary.BreakTransform` (`SceneComponent.K2_GetComponentToWorld` (`self.REF Outside`))))
  ;[0.0625 0.0625 0.0625] Interacting with the door
  (if (not (`self.inside`))
    (set `self.inside` true)
    (`self.K2_SetActorLocationAndRotation` (`GameplayStatics.GetPlayerCharacter` 0) _returnvalue_location _returnvalue_rotation false false)
    (`SceneComponent.K2_SetRelativeRotation` (`self.Door`) (struct :`Yaw` 20.0) false false)
    (else
      (set `self.inside` false)
      (`self.K2_SetActorLocationAndRotation` (`GameplayStatics.GetPlayerCharacter` 0) _returnvalue_location_2 _returnvalue_rotation_2 false false)
      (`SceneComponent.K2_SetRelativeRotation` (`self.Door`) (struct :`Yaw` 90.0) false false))))

(fn `UserConstructionScript`)